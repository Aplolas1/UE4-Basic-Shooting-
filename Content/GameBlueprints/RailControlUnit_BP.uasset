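; RailControlUnit_BP is an interactive control unit that sets a distance and moves a controlled actor along the X axis.
; Traced Up and Down buttons step a clamped distance shown as text.
; Start plays a timeline that lerps the actor from its cached location to that offset from its starting X, triggering an input delay on updates.
; GetCurrentLocation refreshes the cached location used as the lerp origin.
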(event Custom|GetCurrentLocation
  (bind _controlledactor (Variables|FiringRange|GetControlledActor))
  ;[1 1 1] Get Location of Target Follower
  (Utilities|IsValid _controlledactor
    (:Is%20Valid
      (Variables|FiringRange|SetCurrentLocation (Transformation|GetActorLocation _controlledactor)))))

(event EventBeginPlay
  (bind _controlledactor (Variables|FiringRange|GetControlledActor))
  (bind _returnvalue (Transformation|GetActorLocation _controlledactor))
  ;[1 1 1] Set Initial Values on Play
  (Utilities|IsValid _controlledactor
    (:Is%20Valid
      (Variables|FiringRange|SetDefaultLocation _returnvalue)
      (Variables|FiringRange|SetCurrentLocation _returnvalue)
      (Variables|FiringRange|SetDefaultX (.X (Math|Vector|BreakVector _returnvalue))))))

(event Custom|OnTraceDetected
  (params (Component :type Primitive%20Component%20Object%20Reference))
  ;[1 1 1] Handle Interaction with Control Unit Buttons
  (if (Variables|FiringRange|GetInputAllowed)
    (if (== Component (Variables|Default|GetButtonDown))
      (CallFunction|SetDefinedDistance (Utilities|IncrementDistance))
      (elif (== Component (Variables|Default|GetButtonUp))
        (CallFunction|SetDefinedDistance (Utilities|DecrementDistance))
        (elif (== Component (Variables|Default|GetButtonStart))
          (bind _newtrack_0 (Timeline|StartButtonTimeline PlayFromStart)
            (:Update
              (Transformation|SetRelativeLocation (Variables|/Script/Engine.Actor|GetRootComponent (Variables|FiringRange|GetControlledActor)) (Utilities|InterpolatetoPos _newtrack_0) false false)
              (Utilities|AddInputDelay))))))))

(fn ConstructionScript)

(fn SetDefinedDistance
  (params (distance :type Integer))
  (bind _output_get (Variables|FiringRange|SetCurrentDistance distance))
  (Rendering|Components|TextRender|SetText (Variables|Default|GetDefinedDistance) (Utilities|Text|ToText(Integer) _output_get)))