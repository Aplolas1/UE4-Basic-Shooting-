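; DynamicTarget_BP is a spawner actor that sets up a rail-following paper target on BeginPlay.
; SpawnTargetSystem spawns a RailPaperTarget_BP at the world origin and a RailTargetFollower_BP at its own location, then assigns the target as the follower's MovingActor.
; NewMacro_0 duplicates that spawn logic and is not called in this Blueprint.
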(event EventBeginPlay
  (CallFunction|SpawnTargetSystem))

(event Collision|EventActorBeginOverlap
  (params (OtherActor :type Actor%20Object%20Reference)))

(event EventTick
  (params (DeltaSeconds :type Float%20%28single-precision%29)))

(fn ConstructionScript)

(fn SpawnTargetSystem
  (Utilities|FlowControl|Sequence
    (:then_0
      (bind _returnvalue (Game|SpawnActorfromClass "/Game/GameBlueprints/RailPaperTarget_BP.RailPaperTarget_BP_C" (Math|Transform|MakeTransform "0, 0, 0") "AlwaysSpawn" 0 0))
      (Variables|FiringRange|SetTarget _returnvalue))
    (:then_1
      (bind _returnvalue_2 (Game|SpawnActorfromClass "/Game/GameBlueprints/RailTargetFollower_BP.RailTargetFollower_BP_C" (Math|Transform|MakeTransform (Transformation|GetActorLocation)) "Undefined" 0 0))
      (Variables|FiringRange|SetFollower _returnvalue_2))
    (:then_2
      (Variables|/Game/GameBlueprints/RailTargetFollower_BP.RailTargetFollower_BP_C|SetMovingActor (Variables|FiringRange|GetFollower) (Variables|FiringRange|GetTarget)))))